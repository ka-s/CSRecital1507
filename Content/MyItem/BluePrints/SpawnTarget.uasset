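; Target-game manager actor that spawns Glass targets on BeginPlay and tracks hits toward a clear condition.
; SpawnTarget loops up to Many, using random XY within ±Range, fixed height and random yaw, but its loop body runs into a Return node after the first spawn.
; AddHitNum increments HitNum, and Tick sets Text to "CLEAR!" once HitNum reaches Many.
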(event `self.ReceiveBeginPlay`
  (`self.SpawnTarget`))

(event `self.ReceiveTick`
  (params (DeltaSeconds :type "Float (single-precision)"))
  (if (>= (`self.HitNum`) (`self.many`))
    (set `self.Text` "CLEAR!")))

(fn `AddHitNum`
  (set `self.HitNum` (+ (`self.HitNum`) 1)))

(fn `SpawnTarget`
  (bind _range (`self.Range`))
  (bind _returnvalue (* _range -1.0))
  (for _ (range 1 (+ (`self.many`) 1))
    (`|SpawnActorFromClass` "/Game/MyItem/BluePrints/Glass.Glass_C" (`KismetMathLibrary.MakeTransform` (`KismetMathLibrary.MakeVector` (`KismetMathLibrary.RandomFloatInRange` _range _returnvalue) (`KismetMathLibrary.RandomFloatInRange` _range _returnvalue) 200.0) (`KismetMathLibrary.MakeRot` 0.0 (`KismetMathLibrary.RandomFloatInRange` 0.0 180.0))))
    (return))
  (return))

(fn `UserConstructionScript`)