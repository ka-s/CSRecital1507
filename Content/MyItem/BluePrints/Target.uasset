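; Rotating target actor that carries four destructible meshes arranged in a ring around its origin.
; On BeginPlay it gives all four components the same destructible mesh, then places them on the ±X and ±Y axes using Radius and Offset, turning the Y pair 90 degrees.
; A timeline then sets the actor's yaw each update from its track, scaled to a full turn and multiplied by Speed.
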(event `self.ReceiveBeginPlay`
  (`self.SetTargetDes` (`self.Destructible`))
  (`self.SetTargetDesLocation` (`self.Radius`) (`self.Offset`))
  (bind (_direction _track) (`Timeline|TL`)
    (:`Update`
      (`self.SetActorRotation` (`KismetMathLibrary.MakeRot` 0.0 (* (* _track 360.0) (`self.Speed`)))))))

(fn `SetTargetDes`
  (params (StatcMesh :type "DestructibleMesh Object Reference"))
  (`DestructibleComponent.SetDestructibleMesh` (`self.Destructible1`) StatcMesh)
  (`DestructibleComponent.SetDestructibleMesh` (`self.Destructible2`) StatcMesh)
  (`DestructibleComponent.SetDestructibleMesh` (`self.Destructible3`) StatcMesh)
  (`DestructibleComponent.SetDestructibleMesh` (`self.Destructible4`) StatcMesh))

(fn `SetTargetDesLocation`
  (params (Radius :type "Float (double-precision)" :default 0.0) (Offset :type "Float (double-precision)" :default 0.0))
  (bind _returnvalue (* Radius -1.0))
  (bind _destructible3 (`self.Destructible3`))
  (bind _destructible4 (`self.Destructible4`))
  (`SceneComponent.K2_SetRelativeLocation` (`self.Destructible1`) (`KismetMathLibrary.MakeVector` Radius 0.0 Offset) false)
  (`SceneComponent.K2_SetRelativeLocation` (`self.Destructible2`) (`KismetMathLibrary.MakeVector` _returnvalue 0.0 Offset) false)
  (`SceneComponent.K2_SetRelativeLocation` _destructible3 (`KismetMathLibrary.MakeVector` 0.0 Radius Offset) false)
  (`SceneComponent.K2_SetRelativeRotation` _destructible3 (struct :`Yaw` 90.0) false)
  (`SceneComponent.K2_SetRelativeLocation` _destructible4 (`KismetMathLibrary.MakeVector` 0.0 _returnvalue Offset) false)
  (`SceneComponent.K2_SetRelativeRotation` _destructible4 (struct :`Yaw` 90.0) false)
  (return))

(fn `UserConstructionScript`)